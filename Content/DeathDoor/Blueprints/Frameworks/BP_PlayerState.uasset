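; Player state for the hero, tracking owned weapons, health and projectile ammo.
; On BeginPlay it caches the controlled BP_Hero and equips the Sword; weapon updates record the name and refresh the hero's weapon.
; Damage and projectile use decrement their counters, then pass through the Add functions, which cap results at four and call HP and projectile update notifications.
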(event `self.ReceiveBeginPlay`
  (`self.GetOwnerCharacter`)
  (`self.UpdateWeaponData` "Sword"))

(fn `AddHealth`
  (params (PlayerHP :type Integer))
  (locals (Health :type Integer))
  (bind _output_get (set `local.Health` (+ PlayerHP (`self.PlayerHP`))))
  (if (> _output_get 4)
    (set `local.Health` 4))
  (`self.UpdateHP` (`local.Health`)))

(fn `AddProjectileCount`
  (params (ProjectileCount :type Integer))
  (locals (Projectile :type Integer))
  (bind _output_get (set `local.Projectile` (+ ProjectileCount (`self.ProjectileCount`))))
  (if (> _output_get 4)
    (set `local.Projectile` 4))
  (`self.UpdateProjectile` (`local.Projectile`)))

(fn `GetDamage`
  (bind _output_get (set `self.PlayerHP` (- (`self.PlayerHP`) 1)))
  (`self.AddHealth` _output_get))

(fn `GetOwnerCharacter`
  (bind _asbp_hero (cast `/Game/DeathDoor/Blueprints/Characters/BP_Hero` (`Controller.K2_GetPawn` (`GameplayStatics.GetPlayerController` 0))))
  (set `self.OwnerCharacter` _asbp_hero))

(fn `UpdateWeaponData`
  (params (NewWeaponName :type Name))
  (`|ExecutionSequence`
    (:`then_0`
      (`KismetArrayLibrary.Array_AddUnique` (`self.OwnedWeaponName`) (`local.NewWeaponName`)))
    (:`then_1`
      (bind _output_get (set `self.CurrentWeaponRowName` (`local.NewWeaponName`)))
      (`/Game/DeathDoor/Blueprints/Characters/BP_Hero.RefreshWeapon` (`self.OwnerCharacter`) _output_get))))

(fn `UseProjectile`
  (if (>= (`self.ProjectileCount`) 1)
    (bind _output_get (set `self.ProjectileCount` (- (`self.ProjectileCount`) 1)))
    (`self.AddProjectileCount` _output_get)))

(fn `UserConstructionScript`)