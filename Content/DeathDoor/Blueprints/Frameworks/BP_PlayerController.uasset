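; Player controller for the hero in a Death Door-style game, translating Enhanced Input into hero actions.
; On BeginPlay it shows the cursor, caches the possessed BP_Hero, adds the default mapping context and creates the main HUD widget.
; Move, roll and look-far call the hero directly, while melee, held heavy attack and cursor-aimed bow shots route to its attack and bow components.
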(event `self.ReceiveBeginPlay`
  (bind _returnvalue (pcsubsystem `EnhancedInputLocalPlayerSubsystem` self))
  ;[1 1 1] Init
  (`|ExecutionSequence`
    (:`then_0`
      (set `self.bShowMouseCursor` true))
    (:`then_1`
      (bind _asbp_hero (cast `/Game/DeathDoor/Blueprints/Characters/BP_Hero` (`self.K2_GetPawn`)))
      (set `self.PlayerCharacter` _asbp_hero)
      (`/Engine/EditorBlueprintResources/StandardMacros.IsValid` _returnvalue
        (:`Is Valid`
          (`EnhancedInputSubsystemInterface.AddMappingContext` _returnvalue "/Game/DeathDoor/Input/IMC_Default.IMC_Default" 0 (struct)))))
    (:`then_2`
      (bind _returnvalue_2 (`|CreateWidget` "/Game/DeathDoor/Blueprints/Widget/WBP_Default.WBP_Default_C" self))
      (`UserWidget.AddToViewport` _returnvalue_2 0)
      (`/Game/DeathDoor/Blueprints/Widget/WBP_Default.InitWidget` _returnvalue_2))))

(event `EnhancedInput|/Game/DeathDoor/Input/Actions/IA_Move`
  (params (ActionValue :type "Vector2D Structure") (ElapsedSeconds :type "Float (double-precision)") (TriggeredSeconds :type "Float (double-precision)") (InputAction :type "InputAction Object Reference" :default "/Game/DeathDoor/Input/Actions/IA_Move.IA_Move"))
  ;[1 1 1] Movement
  (:`Triggered`
    (`/Game/DeathDoor/Blueprints/Characters/BP_Hero.Move` (`self.PlayerCharacter`) ActionValue_X ActionValue_Y)))

(event `EnhancedInput|/Game/DeathDoor/Input/Actions/IA_Roll`
  (params (ActionValue :type Boolean) (ElapsedSeconds :type "Float (double-precision)") (TriggeredSeconds :type "Float (double-precision)") (InputAction :type "InputAction Object Reference" :default "/Game/DeathDoor/Input/Actions/IA_Roll.IA_Roll"))
  ;[1 1 1] Roll
  (:`Started`
    (`/Game/DeathDoor/Blueprints/Characters/BP_Hero.Roll` (`self.PlayerCharacter`))))

(event `EnhancedInput|/Game/DeathDoor/Input/Actions/IA_Attack`
  (params (ActionValue :type Boolean) (ElapsedSeconds :type "Float (double-precision)") (TriggeredSeconds :type "Float (double-precision)") (InputAction :type "InputAction Object Reference" :default "/Game/DeathDoor/Input/Actions/IA_Attack.IA_Attack"))
  ;[1 1 1] Attack
  (:`Started`
    (`/Game/DeathDoor/Characters/Components/AttackComponent.DoAttack` (`/Game/DeathDoor/Blueprints/Characters/BP_Hero.AttackComponent` (`self.PlayerCharacter`)))))

(event `EnhancedInput|/Game/DeathDoor/Input/Actions/IA_HeavyAttack`
  (params (ActionValue :type Boolean) (ElapsedSeconds :type "Float (double-precision)") (TriggeredSeconds :type "Float (double-precision)") (InputAction :type "InputAction Object Reference" :default "/Game/DeathDoor/Input/Actions/IA_HeavyAttack.IA_HeavyAttack"))
  (bind _attackcomponent (`/Game/DeathDoor/Blueprints/Characters/BP_Hero.AttackComponent` (`self.PlayerCharacter`)))
  ;[1 1 1] HeavyAttack
  (:`Started`
    (`/Game/DeathDoor/Characters/Components/AttackComponent.DoHeavyAttack` _attackcomponent))
  (:`Completed`
    (`/Game/DeathDoor/Characters/Components/AttackComponent.EndHeavyAttack` _attackcomponent TriggeredSeconds)))

(event `EnhancedInput|/Game/DeathDoor/Input/Actions/IA_LookFar`
  (params (ActionValue :type Boolean) (ElapsedSeconds :type "Float (double-precision)") (TriggeredSeconds :type "Float (double-precision)") (InputAction :type "InputAction Object Reference" :default "/Game/DeathDoor/Input/Actions/IA_LookFar.IA_LookFar"))
  (bind _playercharacter (`self.PlayerCharacter`))
  ;[1 1 1] LookFar
  (:`Triggered`
    (`/Game/DeathDoor/Blueprints/Characters/BP_Hero.LookFar` _playercharacter))
  (:`Canceled`
    (`/Game/DeathDoor/Blueprints/Characters/BP_Hero.ResetSpringArmTargetOffset` _playercharacter :!label _label))
  (:`Completed`
    (goto _label)))

(event `EnhancedInput|/Game/DeathDoor/Input/Actions/IA_BowAction`
  (params (ActionValue :type Boolean) (ElapsedSeconds :type "Float (double-precision)") (TriggeredSeconds :type "Float (double-precision)") (InputAction :type "InputAction Object Reference" :default "/Game/DeathDoor/Input/Actions/IA_BowAction.IA_BowAction"))
  (bind _bowactioncomponent (`/Game/DeathDoor/Blueprints/Characters/BP_Hero.BowActionComponent` (`self.PlayerCharacter`)))
  ;[1 1 1] BowAction
  (:`Triggered`
    (`/Game/DeathDoor/Characters/Components/BowActionComponent.MakeCharacterLookCursor` _bowactioncomponent))
  (:`Started`
    (`/Game/DeathDoor/Characters/Components/BowActionComponent.Aim` _bowactioncomponent))
  (:`Completed`
    (`/Game/DeathDoor/Characters/Components/BowActionComponent.Shoot` (`/Game/DeathDoor/Blueprints/Characters/BP_Hero.BowActionComponent` (`self.PlayerCharacter`)))
    (`/Game/DeathDoor/Blueprints/Characters/BP_Hero.ResetSpringArmTargetOffset` (`self.PlayerCharacter`))))

(fn `UserConstructionScript`)