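; BP_Player is the player character Blueprint, handling a melee-style combo attack.
; The Attack event starts AM_Default_Attack at section Attack1 and resets the combo index, or saves a follow-up input if already attacking while CanCombo is set.
; ComboAttackNext builds a section name from an index to play a montage section, with no montage asset specified in that call.
; Nothing in these graphs calls ComboAttackNext or clears the attack flags.
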(event `Attack`
  (if (`self.IsAttacking`)
    (if (`self.CanCombo`)
      (set `self.SaveCombo` true))
    (else
      (`|ExecutionSequence`
        (:`then_1`
          (set `self.IsAttacking` true))
        (:`then_2`
          (set `self.ComboIndex` 0))
        (:`then_3`
          (`|PlayMontage` (`self.Mesh`) "/Game/DeathDoor/Blueprints/Frameworks/Characters/Player/Animations/AM_Default_Attack.AM_Default_Attack" 1.0 0.0 "Attack1"))))))

(fn `ComboAttack_Next`
  (params (Index :type Integer))
  (`self.PlayAnimMontage` null 1.0 (`KismetStringLibrary.Conv_StringToName` (`KismetStringLibrary.Concat_StrStr` "Attack" (`KismetStringLibrary.Conv_IntToString` Index)))))

(fn `UserConstructionScript`
  (`parent.UserConstructionScript`))