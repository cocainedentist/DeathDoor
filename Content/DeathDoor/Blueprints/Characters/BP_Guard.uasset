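; BP_Guard is a guard character with health that spawns helmet, sword and shield actors onto mesh sockets at BeginPlay.
; Damage lowers health and briefly flashes dynamic material instances created in the construction script; at zero health it changes state and disables capsule collision.
; State and attack-combo changes are broadcast through update calls, with the current state stored on the guard.
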(event `self.ReceiveBeginPlay`
  (set `self.CurrentHealth` (`self.MaxHealth`))
  (`self.UpdateCurrentState` "NewEnumerator1")
  (`|ExecutionSequence`
    (:`then_0`
      (bind _returnvalue (`|SpawnActorFromClass` "/Game/DeathDoor/Characters/Guard/Items/Helmet/BP_GuardHelmet.BP_GuardHelmet_C" (`KismetMathLibrary.MakeTransform` (0.0 0.0 0.0)) "Undefined" "MultiplyWithRoot" null null))
      (`self.K2_AttachToComponent` _returnvalue (`self.Mesh`) "helmetsocket" "SnapToTarget" "SnapToTarget" "SnapToTarget" true))
    (:`then_1`
      (bind _returnvalue_2 (`|SpawnActorFromClass` "/Game/DeathDoor/Characters/Guard/Items/Sword/BP_GuardSword.BP_GuardSword_C" (`KismetMathLibrary.MakeTransform` (0.0 0.0 0.0)) "Undefined" "MultiplyWithRoot" null null))
      (`self.K2_AttachToComponent` _returnvalue_2 (`self.Mesh`) "swordsocket" "SnapToTarget" "SnapToTarget" "SnapToTarget" true))
    (:`then_2`
      (bind _returnvalue_3 (`|SpawnActorFromClass` "/Game/DeathDoor/Characters/Guard/Items/Shield/BP_GuardShield.BP_GuardShield_C" (`KismetMathLibrary.MakeTransform` (0.0 0.0 0.0)) "Undefined" "MultiplyWithRoot" null null))
      (`self.K2_AttachToComponent` _returnvalue_3 (`self.Mesh`) "shieldsocket" "SnapToTarget" "SnapToTarget" "SnapToTarget" true))))

(event `self.ReceiveAnyDamage`
  (params (Damage :type "Float (single-precision)") (DamageType :type "DamageType Object Reference") (InstigatedBy :type "Controller Object Reference") (DamageCauser :type "Actor Object Reference"))
  (if (> (`self.CurrentHealth`) 0.0)
    (`|ExecutionSequence`
      (:`then_0`
        (bind _output_get (set `self.CurrentHealth` (- (`self.CurrentHealth`) Damage)))
        (`KismetSystemLibrary.PrintString` (`KismetStringLibrary.Conv_DoubleToString` _output_get) true true (struct :`R` 1.0 :`B` 0.069554 :`A` 1.0))
        (if (<= (`self.CurrentHealth`) 0.0)
          (`self.UpdateState` "NewEnumerator3")
          (`PrimitiveComponent.SetCollisionEnabled` (`self.CapsuleComponent`) "NoCollision")))
      (:`then_1`
        (`MaterialInstanceDynamic.SetScalarParameterValue` (`self.M_Guard1`) "FlashIntensity" 1.0)
        (`MaterialInstanceDynamic.SetScalarParameterValue` (`self.M_Guard2`) "FlashIntensity" 1.0)
        (`KismetSystemLibrary.Delay` 0.1)
        (`MaterialInstanceDynamic.SetScalarParameterValue` (`self.M_Guard1`) "FlashIntensity" -0.0)
        (`MaterialInstanceDynamic.SetScalarParameterValue` (`self.M_Guard2`) "FlashIntensity" -0.0)))))

(fn `UpdateAttackComb`
  (params (AttackCombo :type Integer))
  (`self.UpdateAttackCombo` AttackCombo))

(fn `UpdateState`
  (params (State :type "/Game/DeathDoor/Characters/Guard/E_GuardState Enum" :default "NewEnumerator1"))
  (bind _output_get (set `self.CurrentState` State))
  (`self.UpdateCurrentState` _output_get))

(fn `UserConstructionScript`
  (bind _mesh (`self.Mesh`))
  (`|ExecutionSequence`
    (:`then_0`
      (bind _returnvalue (`PrimitiveComponent.CreateDynamicMaterialInstance` _mesh 0 null "None"))
      (set `self.M_Guard1` _returnvalue))
    (:`then_1`
      (bind _returnvalue_2 (`PrimitiveComponent.CreateDynamicMaterialInstance` _mesh 0 null "None"))
      (set `self.M_Guard2` _returnvalue_2))))