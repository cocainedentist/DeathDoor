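; Player hero character with camera-relative movement, a dodge roll, socketed weapons and mouse-cursor facing, gated by a CharacterState enum.
; Roll plays a montage while a timeline drives boosted movement, then fires buffered attack, heavy attack or bow inputs through action components.
; Weapons spawn from row names and switch sockets when attacking.
; Spring arm lag changes when falling, and its offset leans toward the cursor's ground-plane intersection or a timed focus object.
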(event `Roll`
  (bind _returnvalue (`self.GetLastMovementInputVector`))
  (if (`self.CanRoll`)
    (switch `/Game/DeathDoor/Blueprints/Characters/E_CharacterState` (`self.CharacterState`)
      (:`NewEnumerator0`
        _)
      (:`NewEnumerator3`
        _))
    (`|ExecutionSequence`
      (:`then_0`
        (set `self.CanRoll` false))
      (:`then_1`
        (set `self.CharacterState` "NewEnumerator2")
        (`|PlayMontage` (`self.Mesh`) "/Game/DeathDoor/Characters/Hero/Animations/AM_Roll.AM_Roll"
          (:`then`
            (if (> (`KismetMathLibrary.VSize` _returnvalue) 0.0)
              (set `self.RollDirection` (`KismetMathLibrary.Vector_NormalUnsafe` _returnvalue))
              (else
                (set `self.RollDirection` (`self.GetActorForwardVector`))))
            (`self.K2_SetActorRotation` (`KismetMathLibrary.MakeRotFromX` (`self.RollDirection`)))
            (set `CharacterMovementComponent.MaxWalkSpeed` 1200.0 (`self.CharacterMovement`))
            (`Timeline|Timeline` :!via `PlayFromStart`
              (:`Update`
                (`self.AddMovementInput` (`self.RollDirection`)))
              (:`Finished`
                (set `CharacterMovementComponent.MaxWalkSpeed` 400.0 (`self.CharacterMovement`))
                (set `self.CharacterState` "NewEnumerator0")
                (`KismetSystemLibrary.Delay` 0.2)
                (set `self.CanRoll` true))))
          (:`OnCompleted`
            (`self.CheckBuffer` :!label _label))
          (:`OnInterrupted`
            (goto _label)))))))

(event `self.ReceiveTick`
  (params (DeltaSeconds :type "Float (single-precision)"))
  (`self.CameraMovement`))

(event `CameraFocusOnObject`
  (params (ObjectLocation :type "Vector Structure"))
  (bind _springarm (`self.SpringArm`))
  (bind (_returnvalue_x _returnvalue_y) (`KismetMathLibrary.BreakVector` (* (- (`KismetMathLibrary.MakeVector` (+ ObjectLocation_X 2000.0) (+ ObjectLocation_Y 2000.0) ObjectLocation_Z) (`self.K2_GetActorLocation`)) 0.2)))
  (set `self.IsCameraEvent` true)
  (`Timeline|Timeline_0` :!via `PlayFromStart`
    (:`Update`
      (set `SpringArmComponent.TargetOffset` (`KismetMathLibrary.VInterpTo` (`SpringArmComponent.TargetOffset` _springarm) (`KismetMathLibrary.MakeVector` _returnvalue_x _returnvalue_y) (`GameplayStatics.GetWorldDeltaSeconds`) 25.0) _springarm))
    (:`Finished`
      (set `self.IsCameraEvent` false)
      (`self.ResetSpringArmTargetOffset`))))

(fn `CameraMovement`
  (bind _springarm (`self.SpringArm`))
  (if (`NavMovementInterface.IsFalling` (`self.CharacterMovement`))
    (set `SpringArmComponent.CameraLagSpeed` 0.5 _springarm)
    (set `SpringArmComponent.CameraLagMaxDistance` 0.0 _springarm)
    (else
      (set `SpringArmComponent.CameraLagSpeed` 3.0 _springarm)
      (set `SpringArmComponent.CameraLagMaxDistance` 1500.0 _springarm))))

(fn `CanMove`
  (returns (CanMove :type Boolean))
  (switch `/Game/DeathDoor/Blueprints/Characters/E_CharacterState` (`self.CharacterState`)
    (:`NewEnumerator0`
      (return true))
    (:`NewEnumerator1`
      _)
    (:`NewEnumerator2`
      _)
    (:`NewEnumerator3`
      _)
    (:`NewEnumerator4`
      _))
  (return false))

(fn `CheckBuffer`
  (`|ExecutionSequence`
    (:`then_0`
      (if (`self.AttackBuffer`)
        (`/Game/DeathDoor/Characters/Hero/Components/AttackComponent.DoAttack` (`self.AttackComponent`))
        (set `self.AttackBuffer` false)))
    (:`then_1`
      (if (`self.BowActionBuffer`)
        (`/Game/DeathDoor/Characters/Hero/Components/BowActionComponent.Aim` (`self.BowActionComponent`))
        (set `self.BowActionBuffer` false)))
    (:`then_2`
      (if (`self.RollHeavyAttackBuffer`)
        (`/Game/DeathDoor/Characters/Hero/Components/AttackComponent.DoHeavyAttack` (`self.AttackComponent`))
        (set `self.RollHeavyAttackBuffer` false)))))

(fn `GetCursorIntersection`
  (returns (Intersection :type "Vector Structure"))
  (bind (_worldlocation _worlddirection) (`PlayerController.DeprojectMousePositionToWorld` (`GameplayStatics.GetPlayerController` 0)))
  (return (`.Intersection` (`KismetMathLibrary.LinePlaneIntersection_OriginNormal` _worldlocation (+ _worldlocation (* _worlddirection 10000.0)) (`self.K2_GetActorLocation`) (0.0 0.0 1.0)))))

(fn `LookAtMouseCursor`
  (bind (_returnvalue_roll _returnvalue_pitch _returnvalue_yaw) (`KismetMathLibrary.BreakRotator` (`KismetMathLibrary.FindLookAtRotation` (`self.K2_GetActorLocation`) (`self.GetCursorIntersection`))))
  (`self.K2_SetActorRotation` (`KismetMathLibrary.MakeRotator` 0.0 0.0 _returnvalue_yaw)))

(fn `LookFar`
  (locals (NewLocalVar :type "Vector Structure" :default (0.0 0.0 0.0)))
  (bind _springarm (`self.SpringArm`))
  (bind (_returnvalue_x _returnvalue_y) (`KismetMathLibrary.BreakVector` (* (- (`self.GetCursorIntersection`) (`self.K2_GetActorLocation`)) 0.2)))
  (if (not (`self.IsCameraEvent`))
    (set `SpringArmComponent.TargetOffset` (`KismetMathLibrary.VInterpTo` (`SpringArmComponent.TargetOffset` _springarm) (`KismetMathLibrary.MakeVector` _returnvalue_x _returnvalue_y) (`GameplayStatics.GetWorldDeltaSeconds`) 25.0) _springarm)))

(fn `Move`
  (params (ActionValueX :type "Float (double-precision)") (ActionValueY :type "Float (double-precision)"))
  (bind (_returnvalue_roll _returnvalue_pitch _returnvalue_yaw) (`KismetMathLibrary.BreakRotator` (`SceneComponent.K2_GetComponentRotation` (`self.Camera`))))
  (bind (_returnvalue_roll_2 _returnvalue_pitch_2 _returnvalue_yaw_2) (`KismetMathLibrary.BreakRotator` (`SceneComponent.K2_GetComponentRotation` (`self.Camera`))))
  (if (`self.CanMove`)
    ;[0.15 0.15 0.15 0.502] LeftRight
    (`self.AddMovementInput` (`KismetMathLibrary.GetRightVector` (`KismetMathLibrary.MakeRotator` 0.0 0.0 _returnvalue_yaw_2)) (`local.ActionValueX`))
    ;[0.15 0.15 0.15 0.502] ForwardBackword
    (`self.AddMovementInput` (`KismetMathLibrary.GetForwardVector` (`KismetMathLibrary.MakeRotator` 0.0 0.0 _returnvalue_yaw)) (`local.ActionValueY`))))

(fn `RefreshWeapon`
  (params (CurrentWeaponRowName :type Name))
  (bind _currentweaponactor (`self.CurrentWeaponActor`)
    (:`then`
      (`self.K2_DestroyActor` _currentweaponactor))
    (:`else`
      _))
  (bind _returnvalue (`|SpawnActorFromClass` "/Game/DeathDoor/Items/Weapons/Blueprints/BP_Weapon.BP_Weapon_C" (`KismetMathLibrary.MakeTransform` (0.0 0.0 0.0)) "Undefined" "MultiplyWithRoot" null (`local.CurrentWeaponRowName`) null))
  (bind _output_get (set `self.CurrentWeaponActor` _returnvalue))
  (`self.K2_AttachToComponent` _output_get (`self.Mesh`) "weaponslot" "SnapToTarget" "SnapToTarget" "SnapToTarget" true))

(fn `ResetSpringArmTargetOffset`
  (set `SpringArmComponent.TargetOffset` (0.0 0.0 0.0) (`self.SpringArm`)))

(fn `UpdateState`
  (params (CharacterState :type "/Game/DeathDoor/Blueprints/Characters/E_CharacterState Enum" :default "NewEnumerator0"))
  (set `self.CharacterState` CharacterState))

(fn `UpdateWeaponAttachment`
  (params (IsAttacking :type "/Game/DeathDoor/Blueprints/Characters/E_CharacterState Enum" :default "NewEnumerator0") (SocketName :type Name))
  (switch `/Game/DeathDoor/Blueprints/Characters/E_CharacterState` IsAttacking
    (:`NewEnumerator0`
      (`self.K2_AttachToComponent` (`self.CurrentWeaponActor`) (`self.Mesh`) "weaponslot" "SnapToTarget" "SnapToTarget" "SnapToTarget" true :!label _label))
    (:`NewEnumerator1`
      (`self.K2_AttachToComponent` (`self.CurrentWeaponActor`) (`self.Mesh`) (`local.SocketName`) "SnapToTarget" "SnapToTarget" "SnapToTarget" true))
    (:`NewEnumerator2`
      (goto _label))
    (:`NewEnumerator3`
      (goto _label))
    (:`NewEnumerator4`
      (goto _label))))

(fn `UserConstructionScript`
  (`parent.UserConstructionScript`))