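; BP_Gate is an environment gate that opens by lowering its body along local Z and closes by returning it to the relative origin.
; OpenGate and CloseGate each play their own timeline, lerping GateBody from its current location to the target and updating IsOpened during playback.
; On BeginPlay, a gate flagged IsOpened runs the opening animation.
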(event `self.ReceiveBeginPlay`
  (if (`self.IsOpened`)
    (`self.OpenGate`)))

(event `OpenGate`
  (bind (_direction _opengate) (`Timeline|Open` :!via `PlayFromStart`)
    (:`Update`
      (`SceneComponent.K2_SetRelativeLocation` (`self.Gate_Body`) (`KismetMathLibrary.VLerp` (`SceneComponent.RelativeLocation` (`self.Gate_Body`)) (0.0 0.0 -2493.0) _opengate) false false)
      (set `self.IsOpened` true))))

(event `CloseGate`
  (bind (_direction _opengate) (`Timeline|Timeline` :!via `PlayFromStart`)
    (:`Update`
      (`SceneComponent.K2_SetRelativeLocation` (`self.Gate_Body`) (`KismetMathLibrary.VLerp` (`SceneComponent.RelativeLocation` (`self.Gate_Body`)) (0.0 0.0 0.0) _opengate) false false)
      (set `self.IsOpened` false))))

(fn `UserConstructionScript`)