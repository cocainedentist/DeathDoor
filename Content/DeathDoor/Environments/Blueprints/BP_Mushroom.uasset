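; BP_Mushroom is a damageable environment mushroom that rewards the attacking player with projectile ammo.
; On any damage, it casts the instigator's player state to BP_PlayerState and adds one to its projectile count.
; It then spawns a red shockwave Niagara effect, hides itself and disables collision, and respawns by restoring both after a ten-second delay.
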(event `self.ReceiveAnyDamage`
  (params (Damage :type "Float (single-precision)") (DamageType :type "DamageType Object Reference") (InstigatedBy :type "Controller Object Reference") (DamageCauser :type "Actor Object Reference"))
  (bind _asbp_player_state (cast `/Game/DeathDoor/Blueprints/Frameworks/BP_PlayerState` (`Controller.PlayerState` InstigatedBy)))
  (`/Game/DeathDoor/Blueprints/Frameworks/BP_PlayerState.AddProjectileCount` _asbp_player_state 1)
  (`|ExecutionSequence`
    (:`then_0`
      ;[1 1 1] 수정
      (`NiagaraFunctionLibrary.SpawnSystemAtLocation` "/Game/DeathDoor/Effects/Explode/VFX/Shockwaves/Particles/Color_Variation/VFX_Shockwave_Red.VFX_Shockwave_Red" (`SceneComponent.K2_GetComponentLocation` (`self.Mushroom`))))
    (:`then_1`
      (`self.SetActorHiddenInGame` true)
      (`self.SetActorEnableCollision` false))
    (:`then_2`
      (`KismetSystemLibrary.Delay` 10.0)
      (`self.SetActorHiddenInGame` false)
      (`self.SetActorEnableCollision` true))))

(fn `UserConstructionScript`)