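; BP_GateSwitch is a damage-activated switch that opens its linked Gate once, when BP_Hero is the damage causer.
; Activation spawns a red Niagara burst, swaps the on/off visuals, sinks the Box via a timeline lerp and focuses the hero's camera on the gate.
; BeginPlay resets it to the raised state, while SetActivated snaps it to the pressed state without effects or opening the gate.
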(event `AvtivateSwitch`
  (`NiagaraFunctionLibrary.SpawnSystemAtLocation` "/Game/DeathDoor/Effects/Burst/01_Niagara_Systems/NS_RedBurst.NS_RedBurst" (`SceneComponent.K2_GetComponentLocation` (`self.Box`)))
  (`/Game/DeathDoor/Environments/Blueprints/BP_Gate.OpenGate` (`self.Gate`))
  (`SceneComponent.SetVisibility` (`self.Switch_Off`) true false)
  (`SceneComponent.SetHiddenInGame` (`self.Switch_On`) true false)
  (bind (_direction _opengate) (`Timeline|Timeline` :!via `PlayFromStart`)
    (:`Update`
      (`SceneComponent.K2_SetRelativeLocation` (`self.Box`) (`KismetMathLibrary.VLerp` (`SceneComponent.RelativeLocation` (`self.Box`)) (0.0 0.0 -25.0) _opengate) false false)
      (set `self.IsActivated` true))))

(event `self.ReceiveBeginPlay`
  (`self.ResetSwitch`))

(event `self.ReceiveAnyDamage`
  (params (Damage :type "Float (single-precision)") (DamageType :type "DamageType Object Reference") (InstigatedBy :type "Controller Object Reference") (DamageCauser :type "Actor Object Reference"))
  (bind _asbp_hero (cast `/Game/DeathDoor/Blueprints/Characters/BP_Hero` DamageCauser))
  (if (not (`self.IsActivated`))
    (`self.AvtivateSwitch`)
    (`/Game/DeathDoor/Blueprints/Characters/BP_Hero.CameraFocusOnObject` _asbp_hero (`SceneComponent.K2_GetComponentLocation` (`/Game/DeathDoor/Environments/Blueprints/BP_Gate.Gate_Bottom` (`self.Gate`))))))

(fn `ResetSwitch`
  (`SceneComponent.K2_SetRelativeLocation` (`self.Box`) (0.0 0.0 36.0) false false)
  (`SceneComponent.SetVisibility` (`self.Switch_Off`) false false))

(fn `SetActivated`
  (`SceneComponent.SetVisibility` (`self.Switch_Off`) true false)
  (`SceneComponent.SetVisibility` (`self.Switch_On`) false false)
  (`SceneComponent.K2_SetRelativeLocation` (`self.Box`) (0.0 0.0 -25.0) false false)
  (set `self.IsActivated` true))

(fn `UserConstructionScript`)