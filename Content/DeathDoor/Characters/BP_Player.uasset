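; BP_Player is the player character, with a following camera and a two-swing melee attack.
; Tick pins the spring arm to the character's X and Y at a fixed height, so the camera ignores vertical movement.
; Each attack launches the character forward and alternates two montages.
; A restarting timeline clears the combo count when it finishes; reaching three hits adds a short recovery delay before attacking again.
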(event `self.ReceiveTick`
  (params (DeltaSeconds :type "Float (single-precision)"))
  (bind (_returnvalue_x _returnvalue_y) (`KismetMathLibrary.BreakVector` (`self.K2_GetActorLocation`)))
  ;[1 1 1] CameraMovement
  (`SceneComponent.K2_SetWorldLocation` (`self.SpringArm`) (`KismetMathLibrary.MakeVector` _returnvalue_x _returnvalue_y 100.0) false false))

(event `Attack`
  ;[1 1 1] Attack
  (if (not (`self.IsAttacking`))
    (set `self.IsAttacking` true)
    (`self.AttackReaction`)
    (switch `int` (`self.AttackIndex`)
      (:`0`
        (`|PlayMontage` (`self.Mesh`) "/Game/DeathDoor/Blueprints/Characters/Player/Animations/AM_Attack1.AM_Attack1" 1.5
          (:`then`
            (`/Engine/EditorBlueprintResources/StandardMacros.IncrementInt` (`self.AttackIndex`)
              (:`  `
                (`self.ManageComboCount`))))
          (:`OnCompleted`
            (`self.PostAttack`))))
      (:`1`
        (`|PlayMontage` (`self.Mesh`) "/Game/DeathDoor/Blueprints/Characters/Player/Animations/AM_Attack2.AM_Attack2" 1.5
          (:`then`
            (set `self.AttackIndex` 0)
            (`self.ManageComboCount`))
          (:`OnCompleted`
            (`self.PostAttack`)))))))

(event `PostAttack`
  ;[1 1 1] Attack
  ;;[1 1 1] PostAttack
  (if (>= (`self.ComboCount`) 3)
    (`KismetSystemLibrary.Delay` 0.3)
    (set `self.IsAttacking` false)
    (set `self.ComboCount` 0)
    (else
      (set `self.IsAttacking` false))))

(event `ManageComboCount`
  ;[1 1 1] Attack
  ;;[1 1 1] ManageComboCount
  (`/Engine/EditorBlueprintResources/StandardMacros.IncrementInt` (`self.ComboCount`)
    (:`  `
      (`Timeline|Timeline_AddComboCount` :!via `PlayFromStart`
        (:`Finished`
          (set `self.ComboCount` 0))))))

(fn `AttackReaction`
  (`self.LaunchCharacter` (* (`self.GetActorForwardVector`) 1000.0)))

(fn `UserConstructionScript`
  (`parent.UserConstructionScript`))